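; BP_Customer is a bar customer NPC that offers a quest through dialogue and leaves when served or done.
; TalkTo picks the start, in-progress or completed dialogue from the quest's DT_BarQuests row.
; Returned dialogue options start or complete the quest, or send the customer to ExitPoint.
; Progress persists as name-suffixed scene state strings; completion also removes the quest item from the player's inventory.
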(fn ConstructionScript
  (|CallParentFunction))

(fn Talkto
  (params (Instigator :type Actor%20Object%20Reference) (Dialogue :type Name :default "None"))
  (bind _isquestinprogress (CallFunction|IsQuestinProgress (Variables|Default|GetQuest)))
  (if _isquestinprogress
    (bind _dialog (CallFunction|GetQuestinProgressDialog (Variables|Default|GetQuest)))
    (CallFunction|StartDialogueSequence _dialog)
    (return true)
    (else
      (bind _isquestcompleted (CallFunction|IsQuestCompleted (Variables|Default|GetQuest)))
      (if _isquestcompleted
        (bind _dialog_2 (CallFunction|GetQuestCompletedDialog (Variables|Default|GetQuest)))
        (CallFunction|StartDialogueSequence _dialog_2)
        (return true)
        (else
          (bind _dialog_3 (CallFunction|GetQuestStartDialog (Variables|Default|GetQuest)))
          (CallFunction|StartDialogueSequence _dialog_3)
          (return true))))))

(fn OnReturnDialogueOption
  (params (ReturnOption :type String))
  (switch string ReturnOption
    (:Default
      (return true))
    (:Start
      (bind _isquestinprogress (CallFunction|IsQuestinProgress (Variables|Default|GetQuest)))
      (if _isquestinprogress
        _
        (else
          (CallFunction|StartQuest (Variables|Default|GetQuest))))
      (return true))
    (:Complete
      (bind _isquestinprogress_2 (CallFunction|IsQuestinProgress (Variables|Default|GetQuest)))
      (if _isquestinprogress_2
        (CallFunction|CompleteQuest (Variables|Default|GetQuest)))
      (return true))
    (:Done
      (CallFunction|GotoExitPoint)
      (return false))))

(fn IsQuestinProgress
  (params (quest :type Name))
  (bind _returnvalue (Utilities|GetDataTableRow "/Game/GameJam/Blueprints/Gameplay/Quests/DT_BarQuests.DT_BarQuests" quest)
    (:then
      (return (Utilities|Array|ContainsItem (CallFunction|GetSceneStateStrings) (Utilities|String|Append (.Name (Utilities|Struct|BreakQuestStruct _returnvalue)) "(InProgress)"))))
    (:RowNotFound
      (return false))))

(fn IsQuestCompleted
  (params (quest :type Name))
  (bind _returnvalue (Utilities|GetDataTableRow "/Game/GameJam/Blueprints/Gameplay/Quests/DT_BarQuests.DT_BarQuests" quest)
    (:then
      (return (Utilities|Array|ContainsItem (CallFunction|GetSceneStateStrings) (Utilities|String|Append (.Name (Utilities|Struct|BreakQuestStruct _returnvalue)) "(Completed)"))))
    (:RowNotFound
      (return false))))

(fn GetQuestStartDialog
  (params (quest :type Name))
  (bind _returnvalue (Utilities|GetDataTableRow "/Game/GameJam/Blueprints/Gameplay/Quests/DT_BarQuests.DT_BarQuests" quest)
    (:then
      (return (.DialogStart (Utilities|Struct|BreakQuestStruct _returnvalue))))
    (:RowNotFound
      (return "None"))))

(fn GetQuestinProgressDialog
  (params (quest :type Name))
  (bind _returnvalue (Utilities|GetDataTableRow "/Game/GameJam/Blueprints/Gameplay/Quests/DT_BarQuests.DT_BarQuests" quest)
    (:then
      (return (.DialogInProgress (Utilities|Struct|BreakQuestStruct _returnvalue))))
    (:RowNotFound
      (return "None"))))

(fn GetQuestCompletedDialog
  (params (quest :type Name))
  (bind _returnvalue (Utilities|GetDataTableRow "/Game/GameJam/Blueprints/Gameplay/Quests/DT_BarQuests.DT_BarQuests" quest)
    (:then
      (return (.DialogCompleted (Utilities|Struct|BreakQuestStruct _returnvalue))))
    (:RowNotFound
      (return "None"))))

(fn StartQuest
  (params (quest :type Name))
  (bind _returnvalue (Utilities|GetDataTableRow "/Game/GameJam/Blueprints/Gameplay/Quests/DT_BarQuests.DT_BarQuests" quest)
    (:then
      (Default|AddStateStringtoScene (CallFunction|GetSceneManager) "" (Utilities|String|Append (.Name (Utilities|Struct|BreakQuestStruct _returnvalue)) "(InProgress)"))
      (return))
    (:RowNotFound
      (return))))

(fn CompleteQuest
  (params (quest :type Name))
  (bind _returnvalue (Utilities|GetDataTableRow "/Game/GameJam/Blueprints/Gameplay/Quests/DT_BarQuests.DT_BarQuests" quest)
    (:then
      (Default|RemoveInventoryItem (Variables|/Game/PNCTookit/Blueprints/BP_PNCPlayerController.BP_PNCPlayerController_C|GetInventoryComponent (CallFunction|GetPNCPlayerController)) (.ItemName (Utilities|GetClassDefaults (.Item (Utilities|Struct|BreakQuestStruct _returnvalue)))) true)
      (Default|RemoveStateStringfromScene (CallFunction|GetSceneManager) "" (Utilities|String|Append (.Name (Utilities|Struct|BreakQuestStruct _returnvalue)) "(InProgress)"))
      (Default|AddStateStringtoScene (CallFunction|GetSceneManager) "" (Utilities|String|Append (.Name (Utilities|Struct|BreakQuestStruct _returnvalue)) "(Completed)"))
      (CallFunction|GotoExitPoint)
      (return))
    (:RowNotFound
      (return))))

(fn GotoExitPoint
  (CallFunction|MovetoLocation (Transformation|GetActorLocation (Variables|Default|GetexitPoint)))
  (return))