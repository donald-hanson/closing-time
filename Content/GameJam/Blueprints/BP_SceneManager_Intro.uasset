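; Scene manager for the intro level that presents the main menu.
; Its LoadStateFromStrings calls SetupMainMenu, which switches to the Menu input profile, views through IntroCamera1, shows WBP_MainMenu and binds its events, then returns false.
; New Game removes the menu, fades out the audio and opens BarScene after a short delay.
; Resume Game only unbinds its event and removes the menu.
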(event EventBeginPlay
  (|CallParentFunction) ; This node is disabled and will not be called.\nDrag off pins to build functionality.
)

(event Collision|EventActorBeginOverlap
  (params (OtherActor :type Actor%20Object%20Reference)))

(event EventTick
  (params (DeltaSeconds :type Float%20%28single-precision%29)))

(event Custom|SetupMainMenu
  ;[1 1 1] Set the Main Menu state for the scene.
  (Default|SetInputProfile (CallFunction|GetPNCPlayerController) "Menu")
  (Game|Player|SetViewTargetwithBlend (CallFunction|GetPNCPlayerController) (Variables|Default|GetIntroCamera1) 0.0 "VTBlend_Linear" 0.0 false)
  (bind _returnvalue (UserInterface|CreateWidget "/Game/PNCTookit/Blueprints/Widgets/Menus/WBP_MainMenu.WBP_MainMenu_C"))
  (bind _output_get (Variables|Default|SetMainMenuWidgetRef _returnvalue))
  (UserInterface|Viewport|AddtoViewport _output_get 0)
  (EventDispatchers|BindEventtoOnNewGame _output_get (delegate Custom|OnNewGame))
  (EventDispatchers|BindEventtoOnResumeGame (Variables|Default|GetMainMenuWidgetRef) (delegate Custom|OnResumeGame)))

(event Custom|OnNewGame
  ;[1 1 1] Set the Main Menu state for the scene.
  (EventDispatchers|UnbindallEventsfromOnNewGame (Variables|Default|GetMainMenuWidgetRef))
  (Widget|RemovefromParent (Variables|Default|GetMainMenuWidgetRef))
  (Variables|Default|SetMainMenuWidgetRef 0)
  (Audio|Components|Audio|FadeOut (Variables|/Script/Engine.AmbientSound|GetAudioComponent (Variables|Default|GetaudioRef)) 1.0 0.0 "Linear" :!class /Script/Engine.AudioComponent)
  (Utilities|FlowControl|Delay 1.0)
  (Game|OpenLevel(byName) "BarScene"))

(event Custom|OnResumeGame
  ;[1 1 1] Set the Main Menu state for the scene.
  (EventDispatchers|UnbindallEventsfromOnResumeGame (Variables|Default|GetMainMenuWidgetRef))
  (Widget|RemovefromParent (Variables|Default|GetMainMenuWidgetRef))
  (Variables|Default|SetMainMenuWidgetRef 0))

(fn ConstructionScript
  (|CallParentFunction))

(fn LoadStatefromStrings
  (CallFunction|SetupMainMenu)
  (return false))